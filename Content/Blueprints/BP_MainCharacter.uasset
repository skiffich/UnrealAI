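; BP_MainCharacter is the main character Blueprint, adding rotation indicators and audible landings.
; Each Tick, it points two arrow components along the actor rotation and the control rotation, showing both side by side.
; On landing, it plays a sound at its location and reports a noise event there with itself as instigator, so AI hearing can detect it.
; An attack montage node is present but never runs.
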(event EventOnLanded
  (params (Hit :type Hit%20Result%20Structure%20%28by%20ref%29))
  (bind _returnvalue (Transformation|GetActorLocation))
  (Audio|PlaySoundatLocation "/Engine/VREditor/Sounds/UI/Drop_Item_From_ContentBrowser.Drop_Item_From_ContentBrowser" _returnvalue "0, 0, 0" 1.0 1.0 0.0 0 0 0 0)
  (Class|AISenseHearing|ReportNoiseEvent _returnvalue 1.0 self 0.0 "None"))

(event Collision|EventActorBeginOverlap
  (params (OtherActor :type Actor%20Object%20Reference)))

(event EventTick
  (params (DeltaSeconds :type Float%20%28single-precision%29))
  (Transformation|SetWorldRotation (Variables|Default|GetCharacterRotationArrow) (Transformation|GetActorRotation) false false)
  (Transformation|SetWorldRotation (Variables|Default|GetControllerRotationArrow) (Pawn|GetControlRotation :!class /Script/Engine.Pawn) false false))

(event Input|KeyboardEvents|P
  (params (Key :type Key%20Structure :default "None")))

(fn ConstructionScript)