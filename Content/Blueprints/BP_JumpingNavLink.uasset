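; BP_JumpingNavLink is a smart nav link that makes Characters jump across it during navigation.
; When an agent reaches the link, it casts it to Character, calls Jump and launches it toward the destination, overriding its velocity.
; CalculateVelocity solves the ballistic launch velocity from start, destination and JumpDuration, using a hardcoded gravity of 982 rather than reading the world's value.
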(event EventBeginPlay)

(event Collision|EventActorBeginOverlap
  (params (OtherActor :type Actor%20Object%20Reference)))

(event EventTick
  (params (DeltaSeconds :type Float%20%28single-precision%29)))

(event EventSmartLinkReached
  (params (Agent :type Actor%20Object%20Reference) (Destination :type Vector%20%28by%20ref%29 :default "0, 0, 0"))
  (bind _ascharacter (Utilities|Casting|CastToCharacter Agent))
  (Variables|Default|SetAs%20Character _ascharacter)
  (bind _velocity (CallFunction|CalculateVelocity Destination (Transformation|GetActorLocation _ascharacter) (Variables|Default|GetJump%20Duration)))
  (Character|Jump (Variables|Default|GetAs%20Character))
  (Character|LaunchCharacter (Variables|Default|GetAs%20Character) _velocity true true))

(fn ConstructionScript)

(fn CalculateVelocity
  (params (DestinationLocation :type Vector) (StartingLocation :type Vector) (Duration :type Float%20%28double-precision%29))
  (bind (_x _y _z) (Class|KismetMathLibrary|BreakVector3f DestinationLocation))
  (bind (_x_2 _y_2 _z_2) (Class|KismetMathLibrary|BreakVector3f StartingLocation))
  (LocalVariables|SetIn%20Duration Duration)
  (return (Math|Vector|MakeVector (/ (- _x _x_2) (LocalVariables|GetIn%20Duration)) (/ (- _y _y_2) (LocalVariables|GetIn%20Duration)) (/ (- _z (+ _z_2 (* (Math|Float|Square (LocalVariables|GetIn%20Duration)) -0.5 982.0))) (LocalVariables|GetIn%20Duration)))))